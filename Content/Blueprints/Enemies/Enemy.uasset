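; Enemy character that fights the player, driven by AI through a Blackboard seeded with cooldowns and agent name on BeginPlay.
; Projectile damage lowers health and triggers hit-react or death animation, with collision off and a timed lifespan on death.
; A bullet-detection overlap flags searching and records the target position.
; StartShooting fires an AI projectile aimed just above the player's location, driving animation through anim Blueprint flags.
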(event OnComponentBeginOverlap(BulletDetect)
  (params (OverlappedComponent :type Primitive%20Component%20Object%20Reference) (OtherActor :type Actor%20Object%20Reference) (OtherComp :type Primitive%20Component%20Object%20Reference) (OtherBodyIndex :type Integer) (bFromSweep :type Boolean) (SweepResult :type Hit%20Result%20Structure%20%28by%20ref%29))
  (Utilities|Casting|CastToFirstPersonProjectile OtherActor)
  (AI|Components|Blackboard|SetValueasBool (AI|GetBlackboard 0) (Utilities|Name|MakeLiteralName "IsSearching") true)
  (AI|Components|Blackboard|SetValueasVector (AI|GetBlackboard 0) (Utilities|Name|MakeLiteralName "TargetPosition") (.Location (Collision|BreakHitResult SweepResult))))

(event Custom|StartShooting
  (Interface|Shoot)
  (bind _asue4asp_hero_tpp_anim_blueprint (Utilities|Casting|CastToUE4ASP_HeroTPP_AnimBlueprint (Components|SkeletalMesh|GetAnimInstance (Variables|Character|GetMesh))))
  (Variables|/Game/AnimStarterPack/UE4ASP_HeroTPP_AnimBlueprint.UE4ASP_HeroTPP_AnimBlueprint_C|SetShooting _asue4asp_hero_tpp_anim_blueprint false))

(event EventBeginPlay
  (bind _returnvalue (AI|GetBlackboard 0))
  (AI|Components|Blackboard|SetValueasFloat _returnvalue (Utilities|Name|MakeLiteralName "ShootCooldown") (Variables|Default|GetShootCooldown))
  (AI|Components|Blackboard|SetValueasFloat _returnvalue (Utilities|Name|MakeLiteralName "PatrolMovementCooldown") (Variables|Default|GetPatrolMoveCooldown))
  (Class|BlackboardComponent|SetValueasString _returnvalue (Utilities|Name|MakeLiteralName "AgentName") (Variables|Default|GetAgentName)))

(event Game|Damage|EventAnyDamage
  (params (Damage :type Float%20%28single-precision%29) (DamageType :type Damage%20Type%20Object%20Reference) (InstigatedBy :type Controller%20Object%20Reference) (DamageCauser :type Actor%20Object%20Reference))
  (Utilities|Casting|CastToFirstPersonProjectile DamageCauser)
  (Internal|TakeDamage Damage)
  (AI|Components|Blackboard|SetValueasBool (AI|GetBlackboard 0) (Utilities|Name|MakeLiteralName "TakenDamage") true))

(fn ConstructionScript)

(fn TakeDamage
  (params (damage :type Float%20%28single-precision%29))
  ;[1 1 1] Update health
  (bind _output_get (Variables|Default|Sethealth (- (Variables|Default|Gethealth) damage)))
  ;[1 1 1] Check for death
  (if (<= _output_get 0.0)
    ;[1 1 1] Play a random death animation
    (bind _statemachine (Internal|GetAnimStateMachine))
    (Animation|Montage|MontageStop _statemachine 0.0 0)
    (Variables|/Game/AnimStarterPack/UE4ASP_HeroTPP_AnimBlueprint.UE4ASP_HeroTPP_AnimBlueprint_C|SetDying _statemachine true)
    ;[1 1 1] Set the actor's lifetime and disable collision
    (Actor|SetLifeSpan (Variables|Default|GetlifespanAfterDeath))
    (Collision|SetCollisionEnabled (Variables|Collision|GetCapsuleComponent) "NoCollision")
    (Collision|SetCollisionEnabled (Variables|Character|GetMesh) "NoCollision")
    (Audio|PlaySoundatLocation "/Game/FirstPerson/Audio/Death.Death" (Transformation|GetActorLocation) "0, 0, 0" 1.0 1.0 0.0 0 0 0)
    (else
      ;[1 1 1] Play hit react animation
      (bind _statemachine_2 (Internal|GetAnimStateMachine))
      (Variables|/Game/AnimStarterPack/UE4ASP_HeroTPP_AnimBlueprint.UE4ASP_HeroTPP_AnimBlueprint_C|SetHitReact _statemachine_2 true))))

(fn Shoot
  (bind _returnvalue (Game|GetPlayerCharacter 0))
  (bind _returnvalue_2 (Transformation|GetActorLocation))
  (bind _returnvalue_3 (Transformation|GetActorForwardVector))
  (bind _returnvalue_4 (* _returnvalue_3 1e+02))
  (bind _returnvalue_5 (+ _returnvalue_2 _returnvalue_4))
  ;[1 1 1] Don't shoot if we're dead
  (if (not (Interface|IsDead))
    ;[1 1 1] Play shoot animation
    (bind _statemachine (Internal|GetAnimStateMachine))
    (Variables|/Game/AnimStarterPack/UE4ASP_HeroTPP_AnimBlueprint.UE4ASP_HeroTPP_AnimBlueprint_C|SetShooting _statemachine true)
    ;[1 1 1] Spawn the projectile
    (Game|SpawnActorfromClass "/Game/Blueprints/FirstPersonCharacter/AIFirstPersonProjectile.AIFirstPersonProjectile_C" (Math|Transform|MakeTransform _returnvalue_5 (Math|Rotator|FindLookatRotation _returnvalue_5 (+ (Transformation|GetActorLocation _returnvalue) (* (Transformation|GetActorUpVector _returnvalue) 25)))) "AdjustIfPossibleButDontSpawnIfColliding" 0 0)
    (Audio|PlaySoundatLocation "/Game/FirstPerson/Audio/FirstPersonTemplateWeaponFire02.FirstPersonTemplateWeaponFire02" (Transformation|GetActorLocation) "0, 0, 0" 1.0 1.0 0.0 0 0 0) ; Play firing sound
  ))

(fn GetAnimStateMachine
  (bind _asue4asp_hero_tpp_anim_blueprint (Utilities|Casting|CastToUE4ASP_HeroTPP_AnimBlueprint (Components|SkeletalMesh|GetAnimInstance (Variables|Character|GetMesh)))
    (:then
      (return _asue4asp_hero_tpp_anim_blueprint))
    (:CastFailed
      (Development|PrintString "Failed to cast to anim blueprint")
      (return 0))))

(fn IsDead
  (return (<= (Variables|Default|Gethealth) 0.0)))